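; Player controller that creates and feeds the HUD for a WarpStar pawn, running only on the non-authority (Remote) side.
; BeginPlay creates the HUD widget and caches the pawn; Tick re-enters those steps whenever either reference is invalid.
; Each tick it copies the pawn's wavelength, max speed and turn rate to the HUD.
; It also looks up Goal and Timer actors every tick, updating the goal wavelength only while time remains.
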(event `self.ReceiveBeginPlay`
  (`/Engine/EditorBlueprintResources/ActorMacros.Switch Has Authority`
    (:`Remote`
      (bind _returnvalue (`|CreateWidget` "/Game/ui/HUD.HUD_C" :!label _label))
      (`UserWidget.AddToPlayerScreen` _returnvalue 0)
      (set `self.HUD` _returnvalue)
      (bind _aswarp_star (cast `/Game/WarpStar` (`self.K2_GetPawn`) :!label _label_2))
      (set `self.PayerPawn` _aswarp_star))))

(event `self.ReceiveTick`
  (params (DeltaSeconds :type "Float (single-precision)"))
  (bind _payerpawn (`self.PayerPawn`))
  (bind _hud (`self.HUD`))
  (`/Engine/EditorBlueprintResources/ActorMacros.Switch Has Authority`
    (:`Remote`
      (`/Engine/EditorBlueprintResources/StandardMacros.IsValid` (`self.PayerPawn`)
        (:`Is Valid`
          (`/Engine/EditorBlueprintResources/StandardMacros.IsValid` (`self.HUD`)
            (:`Is Valid`
              (set `/Game/ui/HUD.Wavelength` (`/Game/WarpStar.Wavelength` _payerpawn) _hud)
              (set `/Game/ui/HUD.Speed` (`/Game/WarpStar.CurrentMaxSpeed` _payerpawn) _hud)
              (set `/Game/ui/HUD.Turning` (`/Game/WarpStar.TurnRate` _payerpawn) _hud)
              (bind _outactors (`GameplayStatics.GetAllActorsOfClass` "/Game/goal.goal_C"))
              (bind _outactors_2 (`GameplayStatics.GetAllActorsOfClass` "/Game/timer.timer_C"))
              (if (> (`/Game/timer.timeleft` (`KismetArrayLibrary.Array_Get` _outactors_2)) 0.0)
                (set `/Game/ui/HUD.Goal` (`/Game/goal.Wavelength` (`KismetArrayLibrary.Array_Get` _outactors)) (`self.HUD`))))
            (:`Is Not Valid`
              (goto _label))))
        (:`Is Not Valid`
          (goto _label_2))))))

(fn `UserConstructionScript`)